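; Actor for an ejected .50 calibre shell casing that slides out after a shot, then drops as a physics object.
; Fired opens a Tick-fed gate after a short delay, moving the actor along its local Y axis each frame.
; A second delay closes the gate and enables physics and gravity on the shell.
; A Time variable scales both delays and the per-frame offset.
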(event `Fired`
  (bind _time (`self.Time`))
  (bind _50calibre_bullet2_shell (`self.50Calibre_bullet2_Shell`))
  (`KismetSystemLibrary.Delay` (* 0.1 _time))
  (goto _label :!via `Open`))

(event `self.ReceiveTick`
  (params (DeltaSeconds :type "Float (single-precision)"))
  (bind _time (`self.Time`))
  (bind _50calibre_bullet2_shell (`self.50Calibre_bullet2_Shell`))
  (`/Engine/EditorBlueprintResources/StandardMacros.Gate` true :!label _label
    (:`Exit`
      (`|ExecutionSequence`
        (:`then_0`
          (`self.K2_AddActorLocalOffset` (`KismetMathLibrary.MakeVector` 0.0 (* 0.5 _time))))
        (:`then_1`
          (`KismetSystemLibrary.Delay` (/ 0.1 _time))
          (`|ExecutionSequence`
            (:`then_0`
              (goto _label :!via `Close`))
            (:`then_1`
              (`PrimitiveComponent.SetSimulatePhysics` _50calibre_bullet2_shell true)
              (`PrimitiveComponent.SetEnableGravity` _50calibre_bullet2_shell true))))))))

(fn `UserConstructionScript`)
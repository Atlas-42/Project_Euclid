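; 50CalibreBullet is a projectile actor for a .50 calibre round that starts moving when its Fire event is called.
; Fire opens a gate that Tick feeds, so each frame offsets the bullet along local Z, scaled by delta time, Velocity and Time, and spins its yaw by Time.
; The same chain runs into a ten-second Delay, after which the actor destroys itself.
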(event `Fire`
  (bind _time (`self.Time`))
  (goto _label :!via `Open`))

(event `self.ReceiveTick`
  (params (DeltaSeconds :type "Float (single-precision)"))
  (bind _time (`self.Time`))
  (`/Engine/EditorBlueprintResources/StandardMacros.Gate` true :!label _label
    (:`Exit`
      (`self.K2_AddActorLocalOffset` (`KismetMathLibrary.MakeVector` 0.0 0.0 (* DeltaSeconds (* (`self.Velocity`) _time))))
      (`self.K2_AddActorLocalRotation` (`KismetMathLibrary.MakeRotator` 0.0 0.0 (* 2.0 _time)))
      (`KismetSystemLibrary.Delay` 10.0)
      (`self.K2_DestroyActor`))))

(fn `UserConstructionScript`)
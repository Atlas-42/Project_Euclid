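; Player pawn Blueprint for first-person-style control, which sets itself as player 0's view target on BeginPlay.
; Movement axes add input along the actor's forward and right vectors, and MouseX adds controller yaw.
; MouseY pitches the Camera component directly in two sequenced rotations, one checking each ±75-degree limit.
; Inside the limits the input applies twice; pushing past one reverses one rotation, cancelling the other.
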(event `self.ReceiveBeginPlay`
  (`PlayerController.SetViewTargetWithBlend` (`GameplayStatics.GetPlayerController` 0) self 0.0 "VTBlend_Linear" 0.0 false))

(event `InputAxis|LeftRight`
  (params (AxisValue :type "Float (single-precision)"))
  (`self.AddMovementInput` (`KismetMathLibrary.GetRightVector` (`self.K2_GetActorRotation`)) AxisValue))

(event `InputAxis|ForwardBackward`
  (params (AxisValue :type "Float (single-precision)"))
  (`self.AddMovementInput` (`KismetMathLibrary.GetForwardVector` (`self.K2_GetActorRotation`)) AxisValue))

(event `InputAxis|MouseX`
  (params (AxisValue :type "Float (single-precision)"))
  (`self.AddControllerYawInput` AxisValue))

(event `InputAxis|MouseY`
  (params (AxisValue :type "Float (single-precision)"))
  (bind (_returnvalue_roll _returnvalue_pitch) (`KismetMathLibrary.BreakRotator` (`SceneComponent.K2_GetComponentRotation` (`self.Camera`))))
  (`|ExecutionSequence`
    (:`then_0`
      (if (and (<= AxisValue 0.0) (<= _returnvalue_pitch -75.0))
        (`SceneComponent.K2_AddRelativeRotation` (`self.Camera`) (`KismetMathLibrary.MakeRotator` 0.0 (* AxisValue -1.0)) false false :!label _label)
        (else
          (`SceneComponent.K2_AddRelativeRotation` (`self.Camera`) (`KismetMathLibrary.MakeRotator` 0.0 AxisValue) false false :!label _label_2))))
    (:`then_1`
      (if (and (>= AxisValue 0.0) (>= _returnvalue_pitch 75.0))
        (goto _label)
        (else
          (goto _label_2))))))

(fn `UserConstructionScript`)
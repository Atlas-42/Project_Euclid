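; A .50 calibre round actor that pairs bullet and casing child actors and creeps forward until blocked, like a feeding cartridge.
; Each tick a short, mostly upward trace, ignoring magazines and its own parts, nudges it along local X unless another round, bullet or casing is hit.
; Fire stops that movement, then after a random Time-scaled delay triggers both children, destroys its box and plays the shot sound.
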(event `Fire`
  (bind _time (`self.Time`))
  (`|ExecutionSequence`
    (:`then_0`
      (`KismetSystemLibrary.Delay` (`KismetMathLibrary.RandomFloatInRange` (* 1.0 (`self.Time`)) (* 3.0 (`self.Time`))))
      (`|ExecutionSequence`
        (:`then_0`
          (bind _as50calibre_bullet (cast `/Game/Jordan/blueprints/50CalibreBullet` (`ChildActorComponent.ChildActor` (`self.50CalibreBullet`))))
          (set `/Game/Jordan/blueprints/50CalibreBullet.Time` _time _as50calibre_bullet)
          (`/Game/Jordan/blueprints/50CalibreBullet.Fire` _as50calibre_bullet)
          (bind _as50calibre_casing (cast `/Game/Jordan/blueprints/50CalibreCasing` (`ChildActorComponent.ChildActor` (`self.50CalibreCasing`))))
          (set `/Game/Jordan/blueprints/50CalibreCasing.Time` _time _as50calibre_casing)
          (`/Game/Jordan/blueprints/50CalibreCasing.Fired` _as50calibre_casing)
          (`ActorComponent.K2_DestroyComponent` (`self.Box`)))
        (:`then_1`
          (`AudioComponent.Play` (`self.50CalibreShot_Cue`) 0.0))))
    (:`then_1`
      (goto _label_2 :!via `Close`))))

(event `self.ReceiveTick`
  (params (DeltaSeconds :type "Float (single-precision)"))
  (bind _box1 (`self.Box1`))
  (bind _returnvalue (`SceneComponent.K2_GetComponentLocation` _box1))
  (bind (_returnvalue_x _returnvalue_y _returnvalue_z) (`KismetMathLibrary.BreakVector` (`SceneComponent.GetForwardVector` _box1)))
  (`/Engine/EditorBlueprintResources/StandardMacros.Gate` true :!label _label
    (:`Exit`
      (bind _outhit (`KismetSystemLibrary.LineTraceSingle` _returnvalue (+ _returnvalue (* (`KismetMathLibrary.MakeVector` _returnvalue_x _returnvalue_y (+ _returnvalue_z 90.0)) 0.02)) "TraceTypeQuery1" false (`self.Ignore`)))
      (cast `/Game/Jordan/blueprints/50Calibre` (`.HitActor` (`GameplayStatics.BreakHitResult` _outhit))
        (:`CastFailed`
          (cast `/Game/Jordan/blueprints/50CalibreCasing` (`.HitActor` (`GameplayStatics.BreakHitResult` _outhit))
            (:`CastFailed`
              (cast `/Game/Jordan/blueprints/50CalibreBullet` (`.HitActor` (`GameplayStatics.BreakHitResult` _outhit))
                (:`CastFailed`
                  (`/Engine/EditorBlueprintResources/StandardMacros.Gate` false :!label _label_2
                    (:`Exit`
                      (`self.K2_AddActorLocalOffset` (0.5 0.0 0.0)))))))))))))

(event `self.ReceiveBeginPlay`
  (bind _ignore (`self.Ignore`))
  (bind _outactors (`GameplayStatics.GetAllActorsOfClass` "/Game/Jordan/blueprints/50CalibreMagazine.50CalibreMagazine_C"))
  (for _array_element _outactors
    (`KismetArrayLibrary.Array_Add` (`self.Ignore`) _array_element))
  (`KismetArrayLibrary.Array_Add` _ignore self)
  (`KismetArrayLibrary.Array_Add` _ignore (`ChildActorComponent.ChildActor` (`self.50CalibreCasing`)))
  (`KismetArrayLibrary.Array_Add` _ignore (`ChildActorComponent.ChildActor` (`self.50CalibreBullet`)))
  (goto _label :!via `Open`))

(fn `UserConstructionScript`)